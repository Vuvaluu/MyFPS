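; Master weapon Blueprint for a multiplayer FPS, supporting single or auto fire with hitscan or projectile shots.
; The client traces from camera, then from muzzle toward that aim point, looping through a gate and retriggerable delay for auto fire.
; The server applies damage or spawns a projectile from that client-supplied hit, while projectile weapons also spawn one locally.
; Multicast plays sound and effects, with separate owner-only and non-owner muzzle flashes.
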(event Custom|Client_OnWeaponFire
  (bind _bpcharactermasterref (Variables|Default|GetBPCharacterMasterRef))
  (bind _array (Utilities|Array|MakeArray _bpcharactermasterref))
  (bind _fpcam (Variables|/Game/MP_FPS/Characters/Blueprints/BP_Character_Master.BP_Character_Master_C|GetFPCam _bpcharactermasterref))
  (bind _returnvalue (Transformation|GetWorldLocation _fpcam))
  (switch Utilities|FlowControl|Switch|SwitchonE_FiringModes (Variables|Default|GetFiringMode)
    (:NewEnumerator0
      _)
    (:NewEnumerator1
      (Utilities|FlowControl|Sequence
        (:then_0
          (goto _label Open))
        (:then_1
          (Utilities|FlowControl|Gate true :!label _label
            (:Exit
              (Utilities|FlowControl|Sequence
                (:then_0
                  _)
                (:then_1
                  (Utilities|FlowControl|RetriggerableDelay (Variables|Default|GetFireRate))
                  (goto _label)))))))))
  (bind (_outhit _returnvalue_2) (Collision|SphereTraceByChannel _returnvalue (+ _returnvalue (* (Math|Vector|GetForwardVector (Transformation|GetWorldRotation _fpcam)) (Variables|Default|GetSphereTraceRange))) (Variables|Default|GetSphereTraceRadius) "TraceTypeQuery1" false _array "None"))
  (bind (_outhit_2 _returnvalue_3) (Collision|SphereTraceByChannel (Transformation|GetSocketLocation (Variables|Default|GetSK_FP_Weapon) (Variables|Default|GetMuzzleSocketName)) (Math|Vector|SelectVector (.ImpactPoint (Collision|BreakHitResult _outhit)) (.TraceEnd (Collision|BreakHitResult _outhit)) _returnvalue_2) (Variables|Default|GetSphereTraceRadius) "TraceTypeQuery1" false _array "None"))
  (if (Variables|Default|GetIsHitscan?)
    _
    (else
      (CallFunction|ClientShootInfo _outhit_2 _returnvalue_3)))
  (CallFunction|ServerShootInfo _outhit_2 _returnvalue_3))

(event Custom|Client_ShootInfo
  (params (HitResult :type Hit%20Result%20Structure) (Hit :type Boolean))
  (bind (_bblockinghit _binitialoverlap _time _location _impactpoint _normal _impactnormal _physmat _hitactor _hitcomponent _hitbonename _hititem _faceindex _tracestart _traceend) (Collision|BreakHitResult HitResult))
  (bind _muzzlesocketname (Variables|Default|GetMuzzleSocketName))
  (bind _sk_fp_weapon (Variables|Default|GetSK_FP_Weapon))
  (bind _returnvalue (Transformation|GetSocketLocation _sk_fp_weapon _muzzlesocketname))
  (if (not (Variables|Default|GetIsHitscan?))
    (Game|SpawnActorfromClass (Variables|Default|GetTPProjectile) (Math|Transform|MakeTransform _returnvalue (Math|Rotator|FindLookatRotation _returnvalue (Math|Vector|SelectVector _impactpoint _traceend Hit))) "AlwaysSpawn" (Components|GetOwner) (Game|GetInstigator))))

(event Custom|Server_ShootInfo
  (params (HitResult :type Hit%20Result%20Structure) (Hit :type Boolean))
  (bind (_bblockinghit _binitialoverlap _time _location _impactpoint _normal _impactnormal _physmat _hitactor _hitcomponent _hitbonename _hititem _faceindex _tracestart _traceend) (Collision|BreakHitResult HitResult))
  (bind _muzzlesocketname (Variables|Default|GetMuzzleSocketName))
  (bind _sk_tp_weapon (Variables|Default|GetSK_TP_Weapon))
  (bind _returnvalue (Transformation|GetSocketLocation _sk_tp_weapon _muzzlesocketname))
  (if (Variables|Default|GetIsHitscan?)
    (Game|Damage|ApplyDamage (.HitActor (Collision|BreakHitResult HitResult)) (Math|Conversions|ToFloat(Integer) (Variables|Default|GetDamage)) (Game|GetInstigatorController) self)
    (else
      (Game|SpawnActorfromClass (Variables|Default|GetFPProjectile) (Math|Transform|MakeTransform _returnvalue (Math|Rotator|FindLookatRotation _returnvalue (Math|Vector|SelectVector _impactpoint _traceend Hit))) "AlwaysSpawn" (Components|GetOwner) (Game|GetInstigator))))
  (CallFunction|MulticastWeaponFX HitResult Hit))

(event Custom|Server_OffWeaponFire
  (Utilities|FlowControl|Sequence
    (:then_0
      (Utilities|FlowControl|Delay (Variables|Default|GetWeaponCoolDown))
      (Variables|Default|SetIsCooldownActive? false))
    (:then_1
      (CallFunction|MulticastOffWeaponFire))))

(event Custom|Multicast_OffWeaponFire)

(event Custom|Client_OffWeaponFire
  (bind _bpcharactermasterref (Variables|Default|GetBPCharacterMasterRef))
  (bind _array (Utilities|Array|MakeArray _bpcharactermasterref))
  (bind _fpcam (Variables|/Game/MP_FPS/Characters/Blueprints/BP_Character_Master.BP_Character_Master_C|GetFPCam _bpcharactermasterref))
  (bind _returnvalue (Transformation|GetWorldLocation _fpcam))
  (Utilities|FlowControl|Sequence
    (:then_0
      (Utilities|FlowControl|Gate true) ; enters at Close
    )
    (:then_1
      (CallFunction|ServerOffWeaponFire))))

(event Custom|Multicast_WeaponFX
  (params (HitResult :type Hit%20Result%20Structure) (Hit :type Boolean))
  (bind (_bblockinghit _binitialoverlap _time _location _impactpoint _normal) (Collision|BreakHitResult HitResult))
  (bind _sk_fp_weapon (Variables|Default|GetSK_FP_Weapon))
  (bind _muzzlesocketname (Variables|Default|GetMuzzleSocketName))
  (bind _psmuzzleflash (Variables|Default|GetPSMuzzleFlash))
  (Audio|SpawnSoundAttached (Variables|Default|GetFireWeaponSound) _sk_fp_weapon "MuzzleFlash")
  (Utilities|FlowControl|Sequence
    (:then_0
      (bind _returnvalue (Effects|SpawnEmitterAttached _psmuzzleflash _sk_fp_weapon _muzzlesocketname "0.000000, 0, 0" "0, 0, 0" "SnapToTarget"))
      (Rendering|SetOnlyOwnerSee _returnvalue true :!class /Script/Engine.PrimitiveComponent)
      (if (Variables|Default|GetIsHitscan?)
        (if Hit
          (Audio|PlaySoundatLocation (Variables|Default|GetImpactSound) _impactpoint)
          (Effects|SpawnEmitteratLocation (Variables|Default|GetPSImpact) _impactpoint (Math|Rotator|MakeRotfromZ _normal)))))
    (:then_1
      (bind _returnvalue_2 (Effects|SpawnEmitterAttached _psmuzzleflash (Variables|Default|GetSK_TP_Weapon) _muzzlesocketname "0.000000, 0, 0" "0, 0, 0" "SnapToTarget"))
      (Class|PrimitiveComponent|SetOwnerNoSee _returnvalue_2 true))))

(fn ConstructionScript)